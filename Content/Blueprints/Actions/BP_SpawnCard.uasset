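; BP_SpawnCard is an action Blueprint that spawns a card through the game mode.
; It binds handlers to the action's init, update and execute delegates.
; Init packs the owning player, card value, spawn location and rotation into SpawnData, and execute passes that data to the Director's game mode SpawnCard call.
; The update handler is empty, so the action does no per-tick work.
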(event `self.BindDelegates`
  (add `Action.OnActionInit` (delegate `OnActionInit_Event`))
  (add `Action.OnActionUpdate` (delegate `OnActionUpdate_Event`))
  (add `Action.OnActionExecute` (delegate `ActionExecute_Event`)))

(event `OnActionInit_Event`
  (set `self.SpawnData` (make `/Game/ActionData/ST_SpawnData` (`self.playerOwner_`) (`self.cardValue_`) (`self.spawnLocation_`) (`self.spawnRotation_`))))

(event `OnActionUpdate_Event`
  (params (deltaTime :type "Float (single-precision)")))

(event `ActionExecute_Event`
  (`/Game/Blueprints/Architecture/BP_Gamemode.SpawnCard` (`/Game/Blueprints/Architecture/BP_ActionDirector.GetGamemode` (`self.Director`)) (`self.SpawnData`)))