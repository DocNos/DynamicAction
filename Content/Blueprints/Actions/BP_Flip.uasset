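; BP_Flip is an action Blueprint that rotates its affected object to a flipped rotation over the action's duration.
; BindDelegates hooks Update_Event to the action update delegate, which accumulates delta time into the action's current time.
; Each update teleports the actor to a shortest-path rotator lerp from its current rotation, not a stored start, using elapsed time over duration as alpha, so the turn is non-linear.
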(event `Update_Event` :!signature `self.OnActionUpdate`
  (params (deltaTime :type "Float (single-precision)"))
  (bind _affectedobject_ (`self.affectedObject_`))
  (set `self.actionCurrTime_` (+ deltaTime (`self.actionCurrTime_`)))
  (`Actor.K2_SetActorRotation` _affectedobject_ (`KismetMathLibrary.RLerp` (`Actor.K2_GetActorRotation` _affectedobject_) (`self.flippedRotation_`) (/ (`self.actionCurrTime_`) (`self.actionDuration_`)) true) true))

(event `self.BindDelegates`
  (add `self.OnActionUpdate` (delegate `Update_Event`)))