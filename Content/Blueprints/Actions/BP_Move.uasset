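; BP_Move is an action Blueprint that moves its AffectedObject over the action's duration.
; BindDelegates hooks Update_Event to the action update, which accumulates elapsed time and teleports the object without sweep.
; The new location comes from slerping the actor's location vector toward the normalized EndPos minus CurrPos direction, with elapsed over duration as alpha.
; CurrPos is recomputed by the same expression after the move; an OnActionInit assignment is left unwired.
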(event `Update_Event`
  (params (deltaTime :type "Float (single-precision)"))
  (bind _affectedobject_ (`self.affectedObject_`))
  (bind _returnvalue (`KismetMathLibrary.Vector_SlerpVectorToDirection` (`Actor.K2_GetActorLocation` _affectedobject_) (`KismetMathLibrary.Normal` (- (`self.endPos_`) (`self.currPos_`))) (/ (`self.actionCurrTime_`) (`self.actionDuration_`))))
  (set `self.actionCurrTime_` (+ deltaTime (`self.actionCurrTime_`)))
  (`Actor.K2_SetActorLocation` _affectedobject_ _returnvalue false true)
  (set `self.currPos_` _returnvalue))

(event `self.BindDelegates`
  (add `self.OnActionUpdate` (delegate `Update_Event`)))