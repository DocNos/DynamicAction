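; Card-game action director that creates and runs animation actions on cards and other objects, such as moves, flips and rotations.
; Init registers Blueprint action classes with the builder and binds director events, passing deal and shuffle actions and completed-sequence cleanup to BP_Gamemode.
; Helpers build actions, execute them and list them in the UI until completion, or create delays and sequences.
; ShiftLeft and ShiftRight both currently offset X negatively.
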(event `Tick_Event`
  (params (deltaTime :type "Float (single-precision)")))

(event `ActionStarted_Event`
  (params (Action :type "Action Object Reference"))
  (bind _asbp_spawn_card (cast `/Game/Blueprints/Actions/BP_SpawnCard` Action))
  (set `/Game/Blueprints/Actions/BP_SpawnCard.Director` self _asbp_spawn_card))

(event `self.ReceiveInit`
  (`self.Init BP_Classes`)
  (add `self.OnDirectorTick` (delegate `Tick_Event`))
  (add `self.OnActionStarted` (delegate `ActionStarted_Event`))
  (add `self.OnActionCompleted` (delegate `ActionCompleted_Event`))
  (add `self.OnSequenceCompleted` (delegate `OnSequenceCompleted_Event`))
  (add `self.OnDirectorRef` (delegate `DirectorRef`))
  (add `self.OnDirectorRef_Shuffle` (delegate `DirectorRef_Shuffle`))
  (`self.SetDebugging` true)
  (add `self.OnDirectorTick` (delegate `OnDirectorTick_Event`))
  (add `self.OnSpawnCard` (delegate `OnSpawnCard_Event`)))

(event `OnDirectorTick_Event`
  (params (deltaTime :type "Float (single-precision)")))

(event `OnSpawnCard_Event`
  (params (SpawnAction :type "Action_SpawnCard Object Reference"))
  (`KismetSystemLibrary.PrintString` "card spawns" true true (struct :`G` 0.66 :`B` 1.0 :`A` 1.0) 0.0))

(event `ActionCompleted_Event`
  (params (Action :type "Action Object Reference"))
  (`/Game/Widgets/WBP_HUD.Remove Action` (`self.UI`) Action)
  (`self.RemoveActive` Action))

(event `OnSequenceCompleted_Event`
  (params (Sequence :type "Sequence Structure (by ref)"))
  (`/Game/Blueprints/Architecture/BP_Gamemode.CleanupSequence` (`self.GetGamemode`) Sequence))

(event `DirectorRef` :!signature `self.OnDirectorRef`
  (params (dealAction :type "Action_Deal Object Reference"))
  (bind _asbp_deal (cast `/Game/Blueprints/Actions/BP_Deal` dealAction))
  (`/Game/Blueprints/Architecture/BP_Gamemode.SetDataHolderRef` (`self.GetGamemode`) _asbp_deal))

(event `DirectorRef_Shuffle` :!signature `self.OnDirectorRef_Shuffle`
  (params (shuffleAction :type "Action_Shuffle Object Reference"))
  (bind _asbp_shuffle (cast `/Game/Blueprints/Actions/BP_Shuffle` shuffleAction))
  (`/Game/Blueprints/Architecture/BP_Gamemode.SetDataHolderRef_Shuffle` (`self.GetGamemode`) _asbp_shuffle))

(fn `AddNewSequence`
  (params (`Index / Owner` :type Integer) (Sequence :type "Array of Action Object Reference") (Type :type "SeqType Enum" :default "DEFAULT") (`Sequence Name` :type String))
  (`self.NewSequence` `Index / Owner` Sequence Type `Sequence Name`))

(fn `CreateDelay`
  (params (`Object to Delay` :type "Actor Object Reference") (PreDelay :type "Float (double-precision)") (Duration :type "Float (double-precision)"))
  (returns (`Delay Action` :type "/Game/Blueprints/Actions/BP_Delay Object Reference"))
  (bind _returnvalue (`ActionBuilder.CreateDelayAction` (`self.getBuilder`) `Object to Delay` null PreDelay Duration))
  (bind _asbp_delay (cast `/Game/Blueprints/Actions/BP_Delay` _returnvalue))
  (return _asbp_delay))

(fn `ExecuteTest`
  (params (Action :type "Action Object Reference")))

(fn `FlipCard`
  (params (Card :type "/Game/Blueprints/Objects/BP_Card Object Reference") (Duration :type "Float (double-precision)"))
  (bind _returnvalue (`ActionBuilder.CreateFlipAction` (`self.getBuilder`) Card Duration))
  (`self.ExecuteAction` (`self.GetDirector`) _returnvalue)
  (`/Game/Widgets/WBP_HUD.List_AddToActive` (`self.UI`) _returnvalue))

(fn `GetGamemode`
  (returns (GM :type "/Game/Blueprints/Architecture/BP_Gamemode Object Reference"))
  (bind _asbp_gamemode (cast `/Game/Blueprints/Architecture/BP_Gamemode` (`GameplayStatics.GetGameMode`)))
  (return _asbp_gamemode))

(fn `Init BP_Classes`
  (bind _returnvalue (`self.getBuilder`))
  (`ActionBuilder.SetMoveClass` _returnvalue "/Game/Blueprints/Actions/BP_Move.BP_Move_C")
  (`ActionBuilder.SetFadeClass` _returnvalue "/Game/Blueprints/Actions/BP_Fade.BP_Fade_C")
  (`ActionBuilder.SetRotateClass` _returnvalue "/Game/Blueprints/Actions/BP_Rotate.BP_Rotate_C")
  (`ActionBuilder.SetFlipClass` _returnvalue "/Game/Blueprints/Actions/BP_Flip.BP_Flip_C")
  (`ActionBuilder.SetDelayClass` _returnvalue "/Game/Blueprints/Actions/BP_Delay.BP_Delay_C")
  (`ActionBuilder.SetSpawnClass` _returnvalue "/Game/Blueprints/Actions/BP_SpawnCard.BP_SpawnCard_C")
  (`self.SetDirectorClass` "BP_ActionDirector_C")
  (`ActionBuilder.SetShuffleClass` _returnvalue "/Game/Blueprints/Actions/BP_Shuffle.BP_Shuffle_C")
  (`ActionBuilder.SetDealClass` _returnvalue "/Game/Blueprints/Actions/BP_Deal.BP_Deal_C"))

(fn `MoveTo`
  (params (Data :type "/Game/Struct/ST_MoveData Structure"))
  (`/Engine/EditorBlueprintResources/StandardMacros.IsValid` Data_AffectedObject_2_AE0633CD4E28C78D9EC6ADA242AB4F1C
    (:`Is Valid`
      (bind _returnvalue (`ActionBuilder.CreateMoveAction` (`self.getBuilder`) Data_AffectedObject_2_AE0633CD4E28C78D9EC6ADA242AB4F1C Data_EndPos_5_2D0D46054D333E4F5497C5BC744BE627 Data_Duration_8_82FCDB80460936E553967F9AC646A932))
      (`self.ExecuteAction` (`self.GetDirector`) _returnvalue)
      (`/Game/Widgets/WBP_HUD.List_AddToActive` (`self.UI`) _returnvalue))))

(fn `RotateCard`
  (params (Card :type "/Game/Blueprints/Objects/BP_Card Object Reference") (`Angle Roll` :type "Float (double-precision)") (`Angle Pitch` :type "Float (double-precision)") (`Angle Yaw` :type "Float (double-precision)") (Duration :type "Float (double-precision)"))
  (bind (_returnvalue_roll _returnvalue_pitch _returnvalue_yaw) (`KismetMathLibrary.BreakRotator` (`SceneComponent.K2_GetComponentRotation` (`/Game/Blueprints/Objects/BP_Card.Top` Card))))
  (bind _returnvalue (`ActionBuilder.CreateRotateAction` (`self.getBuilder`) Card (`KismetMathLibrary.MakeRotator` (+ `Angle Roll` _returnvalue_roll) (+ `Angle Pitch` _returnvalue_pitch) (+ `Angle Yaw` _returnvalue_yaw)) Duration))
  (`self.ExecuteAction` _returnvalue)
  (`/Game/Widgets/WBP_HUD.List_AddToActive` (`self.UI`) _returnvalue))

(fn `ShiftDown`
  (params (`Affected Object` :type "Actor Object Reference") (Duration :type "Float (double-precision)"))
  (bind (_returnvalue_x _returnvalue_y _returnvalue_z) (`KismetMathLibrary.BreakVector` (`Actor.K2_GetActorLocation` `Affected Object`)))
  (`self.MoveTo` (make `/Game/Struct/ST_MoveData` `Affected Object` (`KismetMathLibrary.MakeVector` _returnvalue_x (+ _returnvalue_y -100.0) _returnvalue_z) Duration)))

(fn `ShiftLeft`
  (params (`Affected Object` :type "Actor Object Reference") (Duration :type "Float (double-precision)"))
  (bind (_returnvalue_x _returnvalue_y _returnvalue_z) (`KismetMathLibrary.BreakVector` (`Actor.K2_GetActorLocation` `Affected Object`)))
  (`/Engine/EditorBlueprintResources/StandardMacros.IsValid` `Affected Object`
    (:`Is Valid`
      (`self.MoveTo` (make `/Game/Struct/ST_MoveData` `Affected Object` (`KismetMathLibrary.MakeVector` (+ _returnvalue_x -100.0) _returnvalue_y _returnvalue_z) Duration)))))

(fn `ShiftRight`
  (params (`Affected Object` :type "Actor Object Reference") (Duration :type "Float (double-precision)"))
  (bind (_returnvalue_x _returnvalue_y _returnvalue_z) (`KismetMathLibrary.BreakVector` (`Actor.K2_GetActorLocation` `Affected Object`)))
  (`/Engine/EditorBlueprintResources/StandardMacros.IsValid` `Affected Object`
    (:`Is Valid`
      (`self.MoveTo` (make `/Game/Struct/ST_MoveData` `Affected Object` (`KismetMathLibrary.MakeVector` (+ _returnvalue_x -100.0) _returnvalue_y _returnvalue_z) Duration)))))

(fn `ShiftUp`
  (params (`Affected Object` :type "Actor Object Reference") (Duration :type "Float (double-precision)"))
  (bind (_returnvalue_x _returnvalue_y _returnvalue_z) (`KismetMathLibrary.BreakVector` (`Actor.K2_GetActorLocation` `Affected Object`)))
  (`/Engine/EditorBlueprintResources/StandardMacros.IsValid` `Affected Object`
    (:`Is Valid`
      (`self.MoveTo` (make `/Game/Struct/ST_MoveData` `Affected Object` (`KismetMathLibrary.MakeVector` _returnvalue_x (+ _returnvalue_y 100.0) _returnvalue_z) Duration)))))

(fn `ShuffleCards`)