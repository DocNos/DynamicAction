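; Game mode for a card game that sets up the table and brokers card operations on the deck and player hands.
; On BeginPlay it spawns an angled overhead camera, adds the HUD, and caches the data holder actor, game-instance action director, and deck and hand locations.
; Helper functions spawn stacked deck cards and select or fetch cards, delegating storage and selection state to BP_DataHolder, with the deck treated as player 0.
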(event `self.ReceiveBeginPlay`
  (bind _returnvalue (`GameplayStatics.GetPlayerController` 0))
  (bind _persistentdata_holder (`self.PersistentData_Holder`))
  (bind _returnvalue_2 (`|SpawnActorFromClass` "/Script/Engine.CameraActor" (`KismetMathLibrary.MakeTransform` (-384.0 -57.0 564.0) (`KismetMathLibrary.MakeRotator` 0.0 -60.0)) "Undefined" "MultiplyWithRoot" null null))
  (`PlayerController.SetViewTargetWithBlend` _returnvalue _returnvalue_2 0.0 "VTBlend_Linear" 0.0 false)
  (bind _returnvalue_3 (`|CreateWidget` "/Game/Widgets/WBP_HUD.WBP_HUD_C" _returnvalue))
  (`UserWidget.AddToViewport` _returnvalue_3 0)
  (bind _outactors (`GameplayStatics.GetAllActorsOfClass` "/Game/Blueprints/Objects/BP_DataHolder.BP_DataHolder_C"))
  (for _array_element _outactors
    (set `self.PersistentData_Holder` _array_element)
    (break))
  (set `self.Director` (cast `/Game/Blueprints/Architecture/BP_ActionDirector` (`GameplayStatics.GetGameInstance`) :!pure true))
  (set `self.DeckSpawn` (`self.K2_GetActorLocation` (`/Game/Blueprints/Objects/BP_DataHolder.DeckSpawn` _persistentdata_holder)))
  (set `self.P1_Loc` (`self.K2_GetActorLocation` (`/Game/Blueprints/Objects/BP_DataHolder.P1_Hand` _persistentdata_holder)))
  (set `self.P2_Loc` (`self.K2_GetActorLocation` (`/Game/Blueprints/Objects/BP_DataHolder.P2_Hand` _persistentdata_holder)))
  (set `self.P3_Loc` (`self.K2_GetActorLocation` (`/Game/Blueprints/Objects/BP_DataHolder.P3_Hand` _persistentdata_holder))))

(fn `ChangeDeckSelection`
  (params (Iter :type Integer))
  (returns (CurrIndex :type Integer))
  (bind _persistentdata_holder (`self.PersistentData_Holder`))
  (`/Game/Blueprints/Objects/BP_DataHolder.IterCard_Selection` _persistentdata_holder 0 Iter)
  (return (`/Game/Blueprints/Objects/BP_DataHolder.Deck Index` _persistentdata_holder)))

(fn `GetSelectedCard`
  (params (Player :type Integer))
  (returns (Card :type "/Game/Blueprints/Objects/BP_Card Object Reference"))
  (bind _card (`/Game/Blueprints/Objects/BP_DataHolder.GetSelectedCard` (`self.PersistentData_Holder`) Player))
  (return _card))

(fn `GetTopCard`
  (returns (TopCard :type "/Game/Blueprints/Objects/BP_Card Object Reference"))
  (bind _deckcards (`/Game/Blueprints/Objects/BP_DataHolder.DeckCards` (`self.PersistentData_Holder`)))
  (return (`|GetArrayItem` _deckcards (- (`KismetArrayLibrary.Array_Length` _deckcards) 1))))

(fn `SelectCard`
  (params (Index :type Integer))
  (returns (Card :type "/Game/Blueprints/Objects/BP_Card Object Reference"))
  (return (`|GetArrayItem` (`/Game/Blueprints/Objects/BP_DataHolder.DeckCards` (`self.PersistentData_Holder`)) Index)))

(fn `SelectIndex`
  (params (Index :type Integer))
  (returns (Selection_Index :type Integer))
  (bind _selectedindex (`/Game/Blueprints/Objects/BP_DataHolder.Change Selected Card` (`self.PersistentData_Holder`) 0 Index))
  (return _selectedindex))

(fn `SelectTopCard`)

(fn `SpawnCard`
  (returns (`Card Num` :type Integer) (NewCard :type "/Game/Blueprints/Objects/BP_Card Object Reference"))
  (locals (LastSpawned :type Integer))
  (bind _deckspawn (`self.DeckSpawn`))
  (bind _returnvalue (`|SpawnActorFromClass` "/Game/Blueprints/Objects/BP_Card.BP_Card_C" (`KismetMathLibrary.MakeTransform` _deckspawn (`KismetMathLibrary.MakeRotator` 0.0 0.0 -90.0)) "Undefined" "MultiplyWithRoot" null null))
  (bind _deckindex (`/Game/Blueprints/Objects/BP_DataHolder.AddCardTo` (`self.PersistentData_Holder`) 0 _returnvalue))
  (bind _selection_index (`self.SelectIndex` _deckindex))
  (set `self.DeckSpawn` (+ _deckspawn (0.0 0.0 2.0)))
  (return (+ _selection_index 1) _returnvalue))

(fn `UserConstructionScript`)