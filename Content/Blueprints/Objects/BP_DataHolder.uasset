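; Data holder actor for a card game, storing the deck and three player hands, each with a selected-card index.
; BeginPlay caches deck and hand locations from placed actors.
; Functions switch on player number (0 is the deck) to add cards, read selections or step them within bounds, though player 3 checks against P1's hand.
; GetSpawnData numbers cards and returns spawn data at the deck location, raising the stored location slightly.
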(event `self.ReceiveBeginPlay`
  (set `self.DeckLoc` (`self.K2_GetActorLocation` (`self.DeckSpawn`)))
  (set `self.P1_Loc` (`self.K2_GetActorLocation` (`self.P1_Hand`)))
  (set `self.P2_Loc` (`self.K2_GetActorLocation` (`self.P2_Hand`)))
  (set `self.P3_Loc` (`self.K2_GetActorLocation` (`self.P3_Hand`))))

(fn `AddCardTo`
  (params (PlayerNum :type Integer) (Card :type "/Game/Blueprints/Objects/BP_Card Object Reference"))
  (returns (DeckIndex :type Integer))
  (switch `int` PlayerNum
    (:`0`
      (bind _returnvalue (`KismetArrayLibrary.Array_Add` (`self.DeckCards`) Card))
      (return _returnvalue))
    (:`1`
      (bind _returnvalue_2 (`KismetArrayLibrary.Array_Add` (`self.P1_Cards`) Card))
      (return _returnvalue_2))
    (:`2`
      (bind _returnvalue_3 (`KismetArrayLibrary.Array_Add` (`self.P2_Cards`) Card))
      (return _returnvalue_3))
    (:`3`
      (bind _returnvalue_4 (`KismetArrayLibrary.Array_Add` (`self.P3_Cards`) Card))
      (return _returnvalue_4))))

(fn `Change Selected Card`
  (params (Player :type Integer) (CardIndex :type Integer))
  (returns (SelectedIndex :type Integer))
  (switch `int` Player
    (:`0`
      (if (and (< CardIndex (`KismetArrayLibrary.Array_Length` (`self.DeckCards`))) (>= CardIndex 0))
        (bind _output_get (set `self.Deck Index` CardIndex))
        (return _output_get)
        (else
          (return (`self.Deck Index`)))))
    (:`1`
      (if (and (< CardIndex (`KismetArrayLibrary.Array_Length` (`self.P1_Cards`))) (>= CardIndex 0))
        (bind _output_get_2 (set `self.P1 Index` CardIndex))
        (return _output_get_2)
        (else
          (return (`self.P1 Index`)))))
    (:`2`
      (if (and (< CardIndex (`KismetArrayLibrary.Array_Length` (`self.P2_Cards`))) (>= CardIndex 0))
        (bind _output_get_3 (set `self.P2 Index` CardIndex))
        (return _output_get_3)
        (else
          (return (`self.P2 Index`)))))
    (:`3`
      (if (and (< CardIndex (`KismetArrayLibrary.Array_Length` (`self.P1_Cards`))) (>= CardIndex 0))
        (bind _output_get_4 (set `self.P3 Index` CardIndex))
        (return _output_get_4)
        (else
          (return (`self.P3 Index`)))))))

(fn `GetPlayerPositions`
  (returns (PlayerPos :type "Array of Vector Structure"))
  (locals (pp :type "Array of Vector Structure"))
  (bind _pp (`local.pp`))
  (`KismetArrayLibrary.Array_Add` _pp (`self.P1_Loc`))
  (`KismetArrayLibrary.Array_Add` _pp (`self.P2_Loc`))
  (`KismetArrayLibrary.Array_Add` _pp (`self.P3_Loc`))
  (return (`local.pp`)))

(fn `GetSelectedCard`
  (params (Player :type Integer))
  (returns (Card :type "/Game/Blueprints/Objects/BP_Card Object Reference"))
  (switch `int` Player
    (:`0`
      (return (`|GetArrayItem` (`self.DeckCards`) (`self.Deck Index`))))
    (:`1`
      (return (`|GetArrayItem` (`self.P1_Cards`) (`self.P1 Index`))))
    (:`2`
      (return (`|GetArrayItem` (`self.P2_Cards`) (`self.P2 Index`))))
    (:`3`
      (return (`|GetArrayItem` (`self.P3_Cards`) (`self.P3 Index`))))))

(fn `GetSpawnData`
  (params (PlayerNum :type Integer))
  (returns (`Spawn Data` :type "/Game/ActionData/ST_SpawnData Structure"))
  (locals (Loc_Pre :type "Vector Structure"))
  (bind _deckloc (`self.DeckLoc`))
  (bind _totalcards (`self.TotalCards`))
  (switch `int` PlayerNum
    (:`0`
      (bind _result (`/Engine/EditorBlueprintResources/StandardMacros.IncrementInt` _totalcards)
        (:`  `
          (set `local.Loc_Pre` _deckloc)
          (bind _newz (`self.AddToZ` _deckloc 0.5)
            (:`exec`
              (set `self.DeckLoc` _newz)
              (return (make `/Game/ActionData/ST_SpawnData` 0 _result (`local.Loc_Pre`))))))))
    (:`1`
      (bind _result_2 (`/Engine/EditorBlueprintResources/StandardMacros.IncrementInt` _totalcards)
        (:`  `
          (set `local.Loc_Pre` _deckloc)
          (bind _newz_2 (`self.AddToZ` _deckloc 0.5)
            (:`exec`
              (set `self.P1_Loc` _newz_2)
              (return (make `/Game/ActionData/ST_SpawnData` 1 _result_2 (`local.Loc_Pre`))))))))
    (:`2`
      (bind _result_3 (`/Engine/EditorBlueprintResources/StandardMacros.IncrementInt` _totalcards)
        (:`  `
          (set `local.Loc_Pre` _deckloc)
          (bind _newz_3 (`self.AddToZ` _deckloc 0.5)
            (:`exec`
              (set `self.P2_Loc` _newz_3)
              (return (make `/Game/ActionData/ST_SpawnData` 2 _result_3 (`local.Loc_Pre`))))))))
    (:`3`
      (bind _result_4 (`/Engine/EditorBlueprintResources/StandardMacros.IncrementInt` _totalcards)
        (:`  `
          (bind _output_get (set `local.Loc_Pre` _deckloc))
          (bind _newz_4 (`self.AddToZ` _output_get 0.5)
            (:`exec`
              (set `self.P3_Loc` _newz_4)
              (return (make `/Game/ActionData/ST_SpawnData` 3 _result_4 (`local.Loc_Pre`))))))))))

(fn `IterCard_Selection`
  (params (Player :type Integer) (Iter :type Integer))
  (switch `int` Player
    (:`0`
      (`self.Change Selected Card` Player (+ Iter (`self.Deck Index`))))
    (:`1`
      (`self.Change Selected Card` Player (+ (`self.P1 Index`) Iter)))
    (:`2`
      (`self.Change Selected Card` Player (+ (`self.P2 Index`) Iter)))
    (:`3`
      (`self.Change Selected Card` Player (+ (`self.P3 Index`) Iter)))))

(fn `UserConstructionScript`)